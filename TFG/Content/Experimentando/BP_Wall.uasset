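; BP_Wall is a procedurally generated wall that gets holes carved in it by projectile impacts, using Geometry Script.
; On rebuild, it appends a dimensioned box, densely tessellates it and enables complex-as-simple collision.
; When a Projectile hits, it copies RefMesh into a temporary compute mesh and boolean-subtracts it at the local-space impact point, scaled by projectile speed, then releases the compute meshes.
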(event `self.OnRebuildGeneratedMesh`
  (params (TargetMesh :type "DynamicMesh Object Reference"))
  (bind _returnvalue (`GeometryScriptLibrary_MeshPrimitiveFunctions.AppendBox` TargetMesh (struct) (struct) (`self.Dimension X`) 100.0 (`self.Dimension Z`) 0 0 0 "Base" null))
  (bind _returnvalue_2 (`GeometryScriptLibrary_MeshSubdivideFunctions.ApplyPNTessellation` _returnvalue (struct) 30 null))
  (`DynamicMeshComponent.EnableComplexAsSimpleCollision` (`self.DynamicMeshComponent`))
  (set `self.Target Mesh` _returnvalue_2))

(event `self.DynamicMeshComponent.OnComponentHit`
  (params (HitComponent :type "PrimitiveComponent Object Reference") (OtherActor :type "Actor Object Reference") (OtherComp :type "PrimitiveComponent Object Reference") (NormalImpulse :type "Vector Structure") (Hit :type "HitResult Structure (by ref)"))
  (bind _asprojectile (cast `/Game/VRTemplate/Blueprints/Projectile` OtherActor))
  (bind _returnvalue (`self.AllocateComputeMesh`))
  (bind _returnvalue_2 (`GeometryScriptLibrary_StaticMeshFunctions.CopyMeshFromStaticMesh` (`self.Ref Mesh`) _returnvalue (struct) (struct) null)
    (:`Success`
      (bind _returnvalue_3 (/ (`KismetMathLibrary.VSize` (`self.GetVelocity` _asprojectile)) 18000.0))
      (`GeometryScriptLibrary_MeshBooleanFunctions.ApplyMeshBoolean` (`self.Target Mesh`) (struct) _returnvalue_2 (`KismetMathLibrary.MakeTransform` (`KismetMathLibrary.InverseTransformLocation` (`SceneComponent.K2_GetComponentToWorld` (`self.DynamicMeshComponent`)) Hit_Location) (struct) (`KismetMathLibrary.MakeVector` _returnvalue_3 _returnvalue_3 _returnvalue_3)) "Subtract" (struct) null)
      (`self.ReleaseAllComputeMeshes`))))

(fn `UserConstructionScript`)